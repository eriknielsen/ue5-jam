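; BP_storySelector is a story selector actor that displays its option text and records an enemy or treasure choice when its sphere is overlapped.
; The overlap writes the text to the first SampleUI widget and the choice to BP_ChoiceInstance, the game instance.
; For the Enemy 1 type, the game instance's UpdateEnemy1 flag toggles so successive picks alternate between the two enemy slots.
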(event OnComponentBeginOverlap(Sphere)
  (params (OverlappedComponent :type Primitive%20Component%20Object%20Reference) (OtherActor :type Actor%20Object%20Reference) (OtherComp :type Primitive%20Component%20Object%20Reference) (OtherBodyIndex :type Integer) (bFromSweep :type Boolean) (SweepResult :type Hit%20Result%20Structure%20%28by%20ref%29))
  (bind _newtext (Variables|Default|GetNewText))
  (bind _foundwidgets (Widget|GetAllWidgetsOfClass "/Game/Blueprints/SampleUI.SampleUI_C" true))
  (bind _asbp_choice_instance (Utilities|Casting|CastToBP_ChoiceInstance (Game|GetGameInstance)))
  (switch Utilities|FlowControl|Switch|SwitchonStoryChangeEnum (Variables|Default|GetTypeToUpdate)
    (:NewEnumerator0
      (if (Variables|/Game/Blueprints/BP_ChoiceInstance.BP_ChoiceInstance_C|GetUpdateEnemy1 _asbp_choice_instance)
        (Variables|/Game/Blueprints/BP_ChoiceInstance.BP_ChoiceInstance_C|SetUpdateEnemy1 _asbp_choice_instance false)
        (Variables|/Game/Blueprints/SampleUI.SampleUI_C|SetEnemy_1 (Utilities|Array|Get(acopy) _foundwidgets) _newtext)
        (Variables|/Game/Blueprints/BP_ChoiceInstance.BP_ChoiceInstance_C|SetEnemy1 _asbp_choice_instance (Variables|Default|GetEnemyType))
        (else
          (Variables|/Game/Blueprints/BP_ChoiceInstance.BP_ChoiceInstance_C|SetUpdateEnemy1 _asbp_choice_instance true)
          (Variables|/Game/Blueprints/SampleUI.SampleUI_C|SetEnemy_2 (Utilities|Array|Get(acopy) _foundwidgets) _newtext)
          (Variables|/Game/Blueprints/BP_ChoiceInstance.BP_ChoiceInstance_C|SetEnemy2 _asbp_choice_instance (Variables|Default|GetEnemyType)))))
    (:NewEnumerator9
      (Development|PrintText "Treasure")
      (Variables|/Game/Blueprints/SampleUI.SampleUI_C|SetTreasure (Utilities|Array|Get(acopy) _foundwidgets) _newtext)
      (Variables|/Game/Blueprints/BP_ChoiceInstance.BP_ChoiceInstance_C|SetTreasure _asbp_choice_instance (Variables|Default|GetTreasure)))))

(event EventBeginPlay
  (Rendering|Components|TextRender|SetText (Variables|Default|GetTextRender) (Utilities|Text|ToText(String) (Variables|Default|GetNewText))))

(event Collision|EventActorBeginOverlap
  (params (OtherActor :type Actor%20Object%20Reference)))

(event EventTick
  (params (DeltaSeconds :type Float%20%28single-precision%29)))

(fn ConstructionScript)