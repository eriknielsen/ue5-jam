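; BP_SpawnItem is a spawn point that places one of two treasures based on the choice stored in the game instance.
; On BeginPlay it casts the game instance to BP_ChoiceInstance and switches on its Treasure value.
; It spawns the class of Treasure1 or Treasure2 at its own transform, falling back to the first when the value is None.
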(event EventBeginPlay
  (bind _returnvalue (Transformation|GetActorTransform))
  (bind _asbp_choice_instance (Utilities|Casting|CastToBP_ChoiceInstance (Game|GetGameInstance)))
  (switch Utilities|FlowControl|Switch|SwitchonTreasureEnum (Variables|/Game/Blueprints/BP_ChoiceInstance.BP_ChoiceInstance_C|GetTreasure _asbp_choice_instance)
    (:NewEnumerator0
      (Game|SpawnActorfromClass (Utilities|GetClass (Variables|Default|GetTreasure1)) _returnvalue "Undefined" "MultiplyWithRoot" 0 0 :!label _label))
    (:NewEnumerator1
      (Game|SpawnActorfromClass (Utilities|GetClass (Variables|Default|GetTreasure2)) _returnvalue "Undefined" "MultiplyWithRoot" 0 0))
    (:NewEnumerator3
      (goto _label))))

(event Collision|EventActorBeginOverlap
  (params (OtherActor :type Actor%20Object%20Reference)))

(event EventTick
  (params (DeltaSeconds :type Float%20%28single-precision%29)))

(fn ConstructionScript)