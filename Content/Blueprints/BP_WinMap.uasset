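; BP_WinMap is a countdown actor, apparently for a win map, that sends the player to the ChoiceScene level after five seconds.
; BeginPlay sets TimeLeft, and Tick subtracts delta time from it and shows the rounded value on a TextRender.
; Once TimeLeft drops below zero, Tick calls OpenLevelByName to load ChoiceScene.
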(event EventBeginPlay
  (Variables|Default|SetTimeLeft 5.0))

(event Collision|EventActorBeginOverlap
  (params (OtherActor :type Actor%20Object%20Reference)))

(event EventTick
  (params (DeltaSeconds :type Float%20%28single-precision%29))
  (bind _output_get (Variables|Default|SetTimeLeft (- (Variables|Default|GetTimeLeft) DeltaSeconds)))
  (Rendering|Components|TextRender|SetText (Variables|Default|GetTextRender) (Utilities|Text|ToText(String) (Utilities|String|ToString(Float) (Math|Conversions|ToFloat(Integer) (Math|Float|Round _output_get)))))
  (Math|Float|CompareFloat _output_get 0.0
    (:<
      (Game|OpenLevel(byName) "ChoiceScene"))))

(fn ConstructionScript)