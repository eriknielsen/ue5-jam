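; BP_SpawnGuard is a spawner that places a patrolling guard at its own transform on BeginPlay.
; Spawn reads Enemy1 from BP_ChoiceInstance, the game instance, to pick between the Guard1 and Guard2 references, then spawns an actor of that reference's class.
; If the spawned actor casts to BP_Guard1, it receives the spawner's PatrolPoints.
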(event EventBeginPlay
  (CallFunction|Spawn))

(event Collision|EventActorBeginOverlap
  (params (OtherActor :type Actor%20Object%20Reference)))

(event EventTick
  (params (DeltaSeconds :type Float%20%28single-precision%29)))

(fn ConstructionScript)

(fn Spawn
  (bind _asbp_choice_instance (Utilities|Casting|CastToBP_ChoiceInstance (Game|GetGameInstance)))
  (switch Utilities|FlowControl|Switch|SwitchonEnemyEnum (Variables|/Game/Blueprints/BP_ChoiceInstance.BP_ChoiceInstance_C|GetEnemy1 _asbp_choice_instance)
    (:NewEnumerator0
      (Variables|Default|SetActorToSpawn (Variables|Default|GetGuard1)))
    (:NewEnumerator1
      (Variables|Default|SetActorToSpawn (Variables|Default|GetGuard2))))
  (bind _returnvalue (Game|SpawnActorfromClass (Utilities|GetClass (Variables|Default|GetActorToSpawn)) (Transformation|GetActorTransform) "Undefined" "MultiplyWithRoot" 0 0))
  (bind _asbp_guard_2 (Utilities|Casting|CastToBP_Guard1 _returnvalue))
  (Variables|/Game/Blueprints/BP_Guard1.BP_Guard1_C|SetPatrolPoints _asbp_guard_2 (Variables|Default|GetPatrolPoints)))